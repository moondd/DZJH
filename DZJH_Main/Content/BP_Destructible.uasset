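; BP_Destructible is an actor with a destructible component that stops obstructing pawns and the camera once it fractures.
; BeginPlay binds a handler to the actor fracture event, which sets the component's Pawn and Camera collision responses to Ignore.
; AnyDamage only prints a debug string, and leftover nodes for changing object type, enabling physics and adding force are unconnected.
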(event Custom|CE_OnActorFracture
  (params (HitPoint :type Vector%20%28by%20ref%29) (HitDirection :type Vector%20%28by%20ref%29))
  (bind _destructiblecomponent (Variables|Default|GetDestructibleComponent))
  (Collision|SetCollisionResponsetoChannel _destructiblecomponent "ECC_Pawn" "ECR_Ignore")
  (Collision|SetCollisionResponsetoChannel _destructiblecomponent "ECC_Camera" "ECR_Ignore"))

(event EventBeginPlay
  (EventDispatchers|AssignOnActorFracture (delegate Custom|CE_OnActorFracture)))

(event Collision|EventActorBeginOverlap
  (params (OtherActor :type Actor%20Object%20Reference)))

(event EventTick
  (params (DeltaSeconds :type Float%20%28single-precision%29)))

(event Game|Damage|EventAnyDamage
  (params (Damage :type Float%20%28single-precision%29) (DamageType :type Damage%20Type%20Object%20Reference) (InstigatedBy :type Controller%20Object%20Reference) (DamageCauser :type Actor%20Object%20Reference))
  (Development|PrintString "Hello"))

(fn ConstructionScript)