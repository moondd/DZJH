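; Anim notify that plays footstep sounds matched to the surface under the animated mesh's owner.
; On notify, it line-traces downward from just above the owner's location on the Visibility channel.
; On a hit, it spawns the footstep cue at the impact point, with volume scaled by the owner's speed.
; The hit's physical surface type feeds the cue's integer FootstepType parameter to select the sound.
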(fn ReceivedNotify
  (params (MeshComp :type Skeletal%20Mesh%20Component%20Object%20Reference) (Animation :type Anim%20Sequence%20Base%20Object%20Reference))
  (bind _returnvalue (Components|GetOwner MeshComp))
  (bind _returnvalue_2 (Transformation|GetActorLocation _returnvalue))
  (bind (_outhit _returnvalue_3) (Collision|LineTraceByChannel (+ _returnvalue_2 "0, 0,30.000000") (- _returnvalue_2 "0, 0,180.000000") "TraceTypeQuery1" false 0 "None"))
  (if _returnvalue_3
    (bind _returnvalue_4 (Audio|SpawnSoundatLocation "/Game/Res/Sound/Footstep/Cue_Footstep.Cue_Footstep" (.ImpactPoint (Collision|BreakHitResult _outhit)) "0, 0, 0" (Math|Float|MapRangeClamped (Math|Vector|VectorLength (Transformation|GetVelocity _returnvalue)) 0.0 6e+02 0.01 1.0) 1.0 0.0 0 0))
    (Effects|Components|ParticleSystem|SetIntParameter _returnvalue_4 "FootstepType" (Math|Conversions|ToInteger(Byte) (Collision|GetSurfaceType _outhit)))
    (Audio|Components|Audio|Play _returnvalue_4 0.0)
    (return _returnvalue_3)))