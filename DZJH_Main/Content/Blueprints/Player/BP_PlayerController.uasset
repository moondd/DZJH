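; Player controller that manages the player's UI state, with the B key toggling between no UI and the Pause character menu.
; A state change only proceeds when the new state differs, then stores it and removes any current widget, resetting controller mode.
; Entering Pause on the local controller creates W_PlayerCharacterMenu, adds it to the player screen and switches controller mode on.
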(event EventBeginPlay)

(event EventTick
  (params (DeltaSeconds :type Float%20%28single-precision%29)))

(event Input|KeyboardEvents|B
  (params (Key :type Key%20Structure))
  (:Pressed
    (switch Utilities|FlowControl|Switch|SwitchonE_PlayerUIState (Variables|Default|GetE_PlayerUIState)
      (:NewEnumerator0
        (CallFunction|ChangePlayerUIState "NewEnumerator1"))
      (:NewEnumerator1
        (CallFunction|ChangePlayerUIState "NewEnumerator0")))))

(event Custom|ChangePlayerUIState
  (params (NewPlayerUIState :type E_PlayerUIState%20Enum :default "NewEnumerator0"))
  (bind _e_playeruistate (Variables|Default|GetE_PlayerUIState))
  (if (Utilities|Enum|NotEqual(Enum) _e_playeruistate NewPlayerUIState)
    (CallFunction|OnPlayerUIStateChanged _e_playeruistate NewPlayerUIState)))

(event Custom|OnPlayerUIStateChanged
  (params (Leave :type E_PlayerUIState%20Enum :default "NewEnumerator0") (Enter :type E_PlayerUIState%20Enum :default "NewEnumerator0"))
  (bind _output_get (Variables|Default|SetE_PlayerUIState Enter))
  (Utilities|FlowControl|Sequence
    (:then_0
      (Utilities|IsValid (Variables|Default|GetCurrUserWidget)
        (:Is%20Valid
          (Widget|RemovefromParent (Variables|Default|GetCurrUserWidget))
          (CallFunction|SetPlayerControllerMode false))))
    (:then_1
      (switch Utilities|FlowControl|Switch|SwitchonE_PlayerUIState _output_get
        (:NewEnumerator1
          (if (Pawn|IsLocalPlayerController)
            (bind _returnvalue (UserInterface|CreateWidget "/Game/Widget/W_PlayerCharacterMenu.W_PlayerCharacterMenu_C" self))
            (bind _output_get_2 (Variables|Default|SetCurrUserWidget _returnvalue))
            (UserInterface|Viewport|AddtoPlayerScreen _output_get_2)
            (CallFunction|SetPlayerControllerMode true)))))))

(fn ConstructionScript)