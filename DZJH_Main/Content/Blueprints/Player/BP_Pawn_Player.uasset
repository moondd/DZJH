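; BP_Pawn_Player is a player pawn that lets the player click an actor in the world to possess it.
; BeginPlay caches the BP_PlayerController and shows the mouse cursor.
; A left click deprojects the platform mouse position into a debug-drawn line trace on the Camera channel.
; On a hit, it hides the cursor and passes the hit actor and controller to PossessCharacter.
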(event EventBeginPlay
  (bind _asbp_player_controller (Utilities|Casting|CastToBP_PlayerController (Pawn|GetController)))
  (bind _output_get (Variables|Default|SetPlayerController _asbp_player_controller))
  (Variables|/Script/Engine.PlayerController|SetbShowMouseCursor _output_get true))

(event Collision|EventActorBeginOverlap
  (params (OtherActor :type Actor%20Object%20Reference)))

(event EventTick
  (params (DeltaSeconds :type Float%20%28single-precision%29)))

(event Input|MouseEvents|LeftMouseButton
  (params (Key :type Key%20Structure))
  (bind _playercontroller (Variables|Default|GetPlayerController))
  (:Pressed
    (Utilities|IsValid _playercontroller
      (:Is%20Valid
        (bind _returnvalue (Class|WidgetLayoutLibrary|GetMousePositiononPlatform))
        (bind (_outhit _returnvalue_2) (Collision|LineTraceByChannel (.WorldPosition (Class|GameplayStatics|DeprojectScreentoWorld _playercontroller _returnvalue)) (+ (.WorldPosition (Class|GameplayStatics|DeprojectScreentoWorld _playercontroller _returnvalue)) (* (.WorldDirection (Class|GameplayStatics|DeprojectScreentoWorld _playercontroller _returnvalue)) 1e+04)) "TraceTypeQuery2" false 0 "ForDuration"))
        (if _returnvalue_2
          (Variables|/Script/Engine.PlayerController|SetbShowMouseCursor _playercontroller false)
          (CallFunction|PossessCharacter (.HitActor (Collision|BreakHitResult _outhit)) (Variables|Default|GetPlayerController)))))))

(fn ConstructionScript)