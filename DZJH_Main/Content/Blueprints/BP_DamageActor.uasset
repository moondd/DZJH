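; BP_DamageActor delivers one delayed attack step from a damage data array, as either an area overlap or a bullet.
; Area hits filter characters by enemy list, state, angle and height; bullets can home on LockTarget through a timeline.
; GetHitType resolves hits from target state, defense, attack timing and Core before damage is applied.
; Remaining array entries pass to a spawned BP_DamageController after an area check or bullet impact, chaining multi-stage attacks.
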(event OnComponentBeginOverlap(Sphere)
  (params (OverlappedComponent :type Primitive%20Component%20Object%20Reference) (OtherActor :type Actor%20Object%20Reference) (OtherComp :type Primitive%20Component%20Object%20Reference) (OtherBodyIndex :type Integer) (bFromSweep :type Boolean) (SweepResult :type Hit%20Result%20Structure%20%28by%20ref%29))
  (switch Utilities|FlowControl|Switch|SwitchonE_DamageActorType (Utilities|Struct|BreakS_DamageData (Variables|Default|GetCurrDamageData))
    (:NewEnumerator4
      (bind (_can_ _targetcharacter _fromcharacter) (CallFunction|CanShootDamage OtherActor))
      (if _can_
        (bind (_hittype _d_attacktime) (CallFunction|GetHitType _targetcharacter _fromcharacter))
        (Default|DamagefromOther _targetcharacter (Variables|Default|GetCurrDamageData) _fromcharacter _hittype (Variables|Default|GetSaveAttackTime) _d_attacktime (Variables|Default|GetSaveDamageValue))
        (CallFunction|CreatChildDamageData)
        (Actor|DestroyActor)))))

(event Custom|CreatChildDamageData
  (bind _savecontrollertransform (Variables|Default|GetSaveControllerTransform))
  (bind _damagefromactor (Variables|Default|GetDamageFromActor))
  ;[1 1 1] HasChildDamage
  (if (> (Utilities|Array|Length (Variables|Default|GetChildDamageDataArray)) 0)
    (Game|SpawnActorfromClass "/Game/Blueprints/BP_DamageController.BP_DamageController_C" (Math|Transform|MakeTransform (Transformation|GetActorLocation) (.rotation _savecontrollertransform) (.scale _savecontrollertransform)) "Undefined" _damagefromactor _damagefromactor (Variables|Default|GetChildDamageDataArray) (Variables|Default|GetSaveAttackTime) (Variables|Default|GetLockTarget) (Variables|Default|GetSaveDamageValue) 0)))

(event EventBeginPlay
  (bind _damagedataarray (Variables|Default|GetDamageDataArray))
  (bind _saveattacktime (Variables|Default|GetSaveAttackTime))
  (bind _sphere (Variables|Default|GetSphere))
  (bind _locktarget (Variables|Default|GetLockTarget))
  (bind _output_get (Variables|Default|SetChildDamageDataArray _damagedataarray))
  (Utilities|Array|RemoveIndex _output_get)
  (Variables|Default|SetCurrDamageData (Utilities|Array|Get(acopy) _damagedataarray))
  (Utilities|FlowControl|Delay (.DelayTime (Utilities|Struct|BreakS_DamageData (Variables|Default|GetCurrDamageData))))
  (Utilities|FlowControl|Sequence
    (:then_0
      (switch Utilities|FlowControl|Switch|SwitchonE_DamageActorType (.DamageActorType (Utilities|Struct|BreakS_DamageData (Variables|Default|GetCurrDamageData)))
        (:NewEnumerator0
          (Components|Sphere|SetSphereRadius _sphere (Utilities|Struct|BreakS_DamageData (Variables|Default|GetCurrDamageData)) true)
          (bind (_outactors _returnvalue) (Collision|ComponentOverlapActors _sphere (Transformation|GetActorTransform) (Utilities|Array|MakeArray "ObjectTypeQuery7") "/Script/Engine.Actor" (Utilities|Array|MakeArray (Variables|Default|GetDamageFromActor))))
          (if _returnvalue
            (for _array_element _outactors
              (bind (_returnvalue_2 _outtarget _outfrom) (CallFunction|CanDamage _array_element))
              (if _returnvalue_2
                (bind (_hittype _d_attacktime) (CallFunction|GetHitType _outtarget _outfrom))
                (Utilities|FlowControl|Sequence
                  (:then_0
                    (Default|DamageSpont _outfrom (Variables|Default|GetCurrDamageData) _outtarget _saveattacktime _d_attacktime _hittype))
                  (:then_1
                    (Default|DamagefromOther _outtarget (Variables|Default|GetCurrDamageData) _outfrom _hittype _saveattacktime _d_attacktime (Variables|Default|GetSaveDamageValue))))))))
        (:NewEnumerator4
          ;[1 1 1] 子弹逻辑
          (Components|Sphere|SetSphereRadius (Variables|Default|GetSphere) (.Distence (Utilities|Struct|BreakS_DamageData (Variables|Default|GetCurrDamageData))) true)
          (bind _returnvalue_3 (AddComponent|AddProjectileMovementComponent))
          (Variables|/Script/Engine.MovementComponent|SetVelocity _returnvalue_3 (* (Transformation|GetActorForwardVector) (.Speed (Utilities|Struct|BreakS_DamageData (Variables|Default|GetCurrDamageData)))))
          (if (> (.TrackTime (Utilities|Struct|BreakS_DamageData (Variables|Default|GetCurrDamageData))) 0.0)
            (Components|Timeline|SetPlayRate (Variables|Default|GetBulltTrackTime) (/ 1.0 (.TrackTime (Utilities|Struct|BreakS_DamageData (Variables|Default|GetCurrDamageData)))))
            (Timeline|BulltTrackTime PlayFromStart
              (:Update
                ;[1 1 1] 子弹追踪
                (Utilities|IsValid _locktarget
                  (:Is%20Valid
                    (Transformation|SetActorRotation (Math|Interpolation|RInterpTo (Transformation|GetActorRotation) (Math|Rotator|FindLookatRotation (Transformation|GetActorLocation) (Transformation|GetSocketLocation (Variables|/Script/Engine.Character|GetMesh _locktarget) "Bip001-Spine2")) (Utilities|Time|GetWorldDeltaSeconds) (Math|Interpolation|FInterpTo (Variables|Default|GetCurrTarckRotSpeed) (.TrackRotSpeed (Utilities|Struct|BreakS_DamageData (Variables|Default|GetCurrDamageData))) (Utilities|Time|GetWorldDeltaSeconds) 64.0)))
                    (Utilities|IsValid _returnvalue_3
                      (:Is%20Valid
                        (Variables|/Script/Engine.MovementComponent|SetVelocity _returnvalue_3 (* (Transformation|GetActorForwardVector) (.Speed (Utilities|Struct|BreakS_DamageData (Variables|Default|GetCurrDamageData))))))))))
              (:Finished
                ;[1 1 1] 子弹追踪结束
                (if (> (Utilities|Struct|BreakS_DamageData (Variables|Default|GetCurrDamageData)) 0.0)
                  (Variables|/Script/Engine.MovementComponent|SetVelocity _returnvalue_3 (* (Transformation|GetActorForwardVector) (Utilities|Struct|BreakS_DamageData (Variables|Default|GetCurrDamageData)))))))))))
    (:then_2
      (Utilities|FlowControl|Delay 9.0)
      (Actor|DestroyActor))
    (:then_3
      (switch Utilities|FlowControl|Switch|SwitchonE_DamageActorType (Utilities|Struct|BreakS_DamageData (Variables|Default|GetCurrDamageData))
        (:NewEnumerator0
          (CallFunction|CreatChildDamageData)
          (Actor|DestroyActor))))))

(event Collision|EventActorBeginOverlap
  (params (OtherActor :type Actor%20Object%20Reference)))

(event Collision|EventHit
  (params (MyComp :type Primitive%20Component%20Object%20Reference) (Other :type Actor%20Object%20Reference) (OtherComp :type Primitive%20Component%20Object%20Reference) (bSelfMoved :type Boolean) (HitLocation :type Vector :default "0, 0, 0") (HitNormal :type Vector :default "0, 0, 0") (NormalImpulse :type Vector :default "0, 0, 0") (Hit :type Hit%20Result%20Structure%20%28by%20ref%29))
  (bind _currdamagedata (Variables|Default|GetCurrDamageData))
  (bind _locktarget (Variables|Default|GetLockTarget))
  (bind _trackshootspeed (Utilities|Struct|BreakS_DamageData _currdamagedata))
  (Collision|SetCollisionEnabled (Variables|Default|GetSphere) "NoCollision")
  (CallFunction|CreatChildDamageData)
  (Utilities|FlowControl|Sequence
    (:then_0
      (Timeline|BulltTrackTime Stop
        (:Update
          ;[1 1 1] 子弹追踪
          (Utilities|IsValid _locktarget
            (:Is%20Valid
              (Transformation|SetActorRotation (Math|Interpolation|RInterpTo (Transformation|GetActorRotation) (Math|Rotator|FindLookatRotation (Transformation|GetActorLocation) (Transformation|GetSocketLocation (Variables|/Script/Engine.Character|GetMesh _locktarget) "Bip001-Spine2")) (Utilities|Time|GetWorldDeltaSeconds) (Math|Interpolation|FInterpTo (Variables|Default|GetCurrTarckRotSpeed) (.TrackRotSpeed (Utilities|Struct|BreakS_DamageData (Variables|Default|GetCurrDamageData))) (Utilities|Time|GetWorldDeltaSeconds) 64.0)))
              (Utilities|IsValid (stale EventBeginPlay _returnvalue_3)
                (:Is%20Valid
                  (Variables|/Script/Engine.MovementComponent|SetVelocity (stale EventBeginPlay _returnvalue_3) (* (Transformation|GetActorForwardVector) (.Speed (Utilities|Struct|BreakS_DamageData (Variables|Default|GetCurrDamageData))))))))))
        (:Finished
          ;[1 1 1] 子弹追踪结束
          (if (> _trackshootspeed 0.0)
            (Variables|/Script/Engine.MovementComponent|SetVelocity (stale EventBeginPlay _returnvalue_3) (* (Transformation|GetActorForwardVector) _trackshootspeed))))))
    (:then_1
      (Utilities|FlowControl|Delay 3.0)
      (Actor|DestroyActor))))

(fn ConstructionScript)

(fn FindDamageTarget
  (params (object :type Actor%20Object%20Reference)))

(fn CanDamage
  (params (TargetActor :type Object%20Object%20Reference))
  (bind _returnvalue (Transformation|GetActorLocation))
  (bind _currdamagedata (Variables|Default|GetCurrDamageData))
  (bind (_angle _max_z _min_z) (Utilities|Struct|BreakS_DamageData _currdamagedata))
  (bind _asbp_character_base (Utilities|Casting|CastToBP_Character_Base (Variables|Default|GetDamageFromActor))
    (:then
      (bind _asbp_character_base_2 (Utilities|Casting|CastToBP_Character_Base TargetActor)
        (:then
          (return (Math|Boolean|ANDBoolean (or (Pawn|IsPlayerControlled _asbp_character_base) (Utilities|Array|ContainsItem (Variables|/Game/Blueprints/Character/BP_Character_Base.BP_Character_Base_C|GetEnemyArray _asbp_character_base) _asbp_character_base_2)) (< (Variables|/Game/Blueprints/Character/BP_Character_Base.BP_Character_Base_C|GetCharacterState_Base _asbp_character_base_2) 4) (and (Math|Float|InRange(Float) (Math|Float|Absolute(Float) (.yaw (Math|Rotator|Delta(Rotator) (Math|Rotator|FindLookatRotation _returnvalue (Transformation|GetWorldLocation (Variables|/Script/Engine.Character|GetMesh _asbp_character_base_2))) (Math|Conversions|RotationFromXVector (Transformation|GetActorForwardVector _asbp_character_base))))) 0.0 _angle) (Math|Float|InRange(Float) (- (.Z (Math|Vector|BreakVector (Transformation|GetWorldLocation (Variables|/Script/Engine.Character|GetMesh _asbp_character_base_2)))) (.Z (Math|Vector|BreakVector _returnvalue))) _min_z _max_z))) _asbp_character_base_2 _asbp_character_base))
        (:CastFailed
          _)))
    (:CastFailed
      _))
  (return false 0 0))

(fn GetHitType
  (params (TargetCharacter :type BP%20Character%20Base%20Object%20Reference) (FromCharacter :type BP%20Character%20Base%20Object%20Reference))
  (bind _saveattacktime (Variables|Default|GetSaveAttackTime))
  (bind _output_get (LocalVariables|SetLoc_TargetCharacter TargetCharacter))
  (bind _output_get_2 (LocalVariables|SetLoc_FromCharacter FromCharacter))
  (LocalVariables|SetLoc_CombatValue (Variables|/Game/Blueprints/Character/BP_Character_Base.BP_Character_Base_C|GetCombatValue _output_get_2))
  (LocalVariables|SetLoc_D_AttackTime (- _saveattacktime (Variables|/Game/Blueprints/Character/BP_Character_Base.BP_Character_Base_C|GetCurrAttackTime _output_get)))
  (LocalVariables|SetLoc_DamageData (Variables|Default|GetCurrDamageData))
  (switch Utilities|FlowControl|Switch|SwitchonE_CharacterState_Base (Variables|/Game/Blueprints/Character/BP_Character_Base.BP_Character_Base_C|GetCharacterState_Base _output_get)
    (:NewEnumerator0
      (if (and (Utilities|Enum|Equal(Enum) (Variables|/Game/Blueprints/Character/BP_Character_Base.BP_Character_Base_C|GetCharacterState_Action (LocalVariables|GetLoc_TargetCharacter)) "NewEnumerator2") (Variables|/Game/Blueprints/Character/BP_Character_Base.BP_Character_Base_C|GetIsAttacking? (LocalVariables|GetLoc_TargetCharacter))) :!label _label
        (if (Pawn|IsPlayerControlled (LocalVariables|GetLoc_FromCharacter))
          (return "NewEnumerator7" 1.0)
          (else
            (return "NewEnumerator12" (LocalVariables|GetLoc_D_AttackTime))))
        (elif (or (> (Variables|/Game/Blueprints/Character/BP_Character_Base.BP_Character_Base_C|GetDefenseTime (LocalVariables|GetLoc_TargetCharacter)) 0.0) (Default|AutoDefense (LocalVariables|GetLoc_TargetCharacter) (LocalVariables|GetLoc_CombatValue)))
          (if (Math|Boolean|ANDBoolean (Utilities|Enum|Equal(Enum) (.DamageType (Utilities|Struct|BreakS_DamageData (LocalVariables|GetLoc_DamageData))) "NewEnumerator0") (<= (Variables|/Game/Blueprints/Character/BP_Character_Base.BP_Character_Base_C|GetCurrEnergy (LocalVariables|GetLoc_FromCharacter)) 0.0) (Pawn|IsPlayerControlled (LocalVariables|GetLoc_FromCharacter)) (Utilities|Enum|NotEqual(Enum) (.DamageActorType (Utilities|Struct|BreakS_DamageData (LocalVariables|GetLoc_DamageData))) "NewEnumerator4"))
            (return "NewEnumerator1" (LocalVariables|GetLoc_D_AttackTime))
            (else
              (return "NewEnumerator0" (LocalVariables|GetLoc_D_AttackTime))))
          (elif (<= (Variables|/Game/Blueprints/Character/BP_Character_Base.BP_Character_Base_C|GetDefenseTime (LocalVariables|GetLoc_TargetCharacter)) 0.0)
            (if (> (LocalVariables|GetLoc_D_AttackTime) 0.0)
              (if (<= (Variables|/Game/Blueprints/Character/BP_Character_Base.BP_Character_Base_C|GetCurrCore (LocalVariables|GetLoc_TargetCharacter)) 0.0)
                (Utilities|FlowControl|Sequence
                  (:then_0
                    _)
                  (:then_1
                    (return "NewEnumerator6" (LocalVariables|GetLoc_D_AttackTime))))
                (else
                  (Variables|/Game/Blueprints/Character/BP_Character_Base.BP_Character_Base_C|SetCurrCore (LocalVariables|GetLoc_TargetCharacter) (- (Variables|/Game/Blueprints/Character/BP_Character_Base.BP_Character_Base_C|GetCurrCore (LocalVariables|GetLoc_TargetCharacter)) (Math|Float|SelectFloat 0.0 (LocalVariables|GetLoc_D_AttackTime) (< (LocalVariables|GetLoc_D_AttackTime) 0.0))))
                  (return "NewEnumerator10" (LocalVariables|GetLoc_D_AttackTime))))
              (else
                (return "NewEnumerator10" (LocalVariables|GetLoc_D_AttackTime))))
            (else
              (return "NewEnumerator5" _saveattacktime))))))
    (:NewEnumerator1
      (goto _label))
    (:NewEnumerator13
      (return "NewEnumerator8" _saveattacktime))
    (:NewEnumerator14
      (if (Pawn|IsPlayerControlled (LocalVariables|GetLoc_TargetCharacter))
        (return "NewEnumerator8" _saveattacktime)
        (else
          (return "NewEnumerator6" (LocalVariables|GetLoc_D_AttackTime)))))
    (:NewEnumerator4
      (return "NewEnumerator10" 0.0))
    (:NewEnumerator15
      (return "NewEnumerator11" _saveattacktime)))
  (Variables|/Game/Blueprints/Character/BP_Character_Base.BP_Character_Base_C|SetCurrCore (LocalVariables|GetLoc_TargetCharacter) (Utilities|Struct|BreakS_CharacterData (Variables|/Game/Blueprints/Character/BP_Character_Base.BP_Character_Base_C|GetCharacterData (LocalVariables|GetLoc_TargetCharacter)))))

(fn CanShootDamage
  (params (Actor :type Actor%20Object%20Reference))
  (bind _damagedactorarray (Variables|Default|GetDamagedActorArray))
  (bind _damagefromactor (Variables|Default|GetDamageFromActor))
  (if (!= Actor _damagefromactor)
    (if (Utilities|Array|ContainsItem _damagedactorarray Actor)
      _
      (else
        (Utilities|Array|Add _damagedactorarray Actor)
        (bind _asbp_character_base (Utilities|Casting|CastToBP_Character_Base Actor)
          (:then
            (bind _asbp_character_base_2 (Utilities|Casting|CastToBP_Character_Base _damagefromactor)
              (:then
                (return (Utilities|Enum|NotEqual(Enum) (Variables|/Game/Blueprints/Character/BP_Character_Base.BP_Character_Base_C|GetCharacterState_Base _asbp_character_base) "NewEnumerator4") _asbp_character_base _asbp_character_base_2))
              (:CastFailed
                _)))
          (:CastFailed
            _)))))
  (return false 0 0))