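; BP_OrientNotify is an animation notify state that controls a BP_Character_Base's attack orientation during a montage or animation window.
; On begin, it refreshes the owner's saved attack vector and copies the notify's OrientSpeed to the character.
; On tick, it refreshes that vector again only when the Update flag is set, allowing either a one-time snapshot or continuous re-aiming.
; It has no end handler, so OrientSpeed is not reset here.
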(fn ReceivedNotifyBegin
  (params (MeshComp :type Skeletal%20Mesh%20Component%20Object%20Reference) (Animation :type Anim%20Sequence%20Base%20Object%20Reference) (TotalDuration :type Float%20%28single-precision%29))
  (bind _asbp_character_base (Utilities|Casting|CastToBP_Character_Base (Components|GetOwner MeshComp))
    (:then
      (Default|RefreshSaveAttackVector _asbp_character_base)
      (Variables|/Game/Blueprints/Character/BP_Character_Base.BP_Character_Base_C|SetOrientSpeed _asbp_character_base (Variables|Default|GetOrientSpeed))
      (return true))
    (:CastFailed
      (return false))))

(fn ReceivedNotifyTick
  (params (MeshComp :type Skeletal%20Mesh%20Component%20Object%20Reference) (Animation :type Anim%20Sequence%20Base%20Object%20Reference) (FrameDeltaTime :type Float%20%28single-precision%29))
  (if (Variables|Default|GetUpdate?)
    (bind _asbp_character_base (Utilities|Casting|CastToBP_Character_Base (Components|GetOwner MeshComp))
      (:then
        (Default|RefreshSaveAttackVector _asbp_character_base)
        (return true))
      (:CastFailed
        (return false)))))