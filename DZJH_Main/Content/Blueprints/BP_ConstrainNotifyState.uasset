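; Animation notify state that sets a movement plane constraint on the owning BP_Character_Base while the notify window plays.
; Each tick it sets the CharacterMovement plane constraint normal to the actor's current right vector, describing a forward-up plane that follows the character's facing.
; When the notify ends, it resets the normal to zero to clear the constraint.
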(fn ReceivedNotifyTick
  (params (MeshComp :type Skeletal%20Mesh%20Component%20Object%20Reference) (Animation :type Anim%20Sequence%20Base%20Object%20Reference) (FrameDeltaTime :type Float%20%28single-precision%29))
  (bind _asbp_character_base (Utilities|Casting|CastToBP_Character_Base (Components|GetOwner MeshComp))
    (:then
      (Class|MovementComponent|SetPlaneConstraintNormal (Variables|/Script/Engine.Character|GetCharacterMovement _asbp_character_base) (Transformation|GetActorRightVector _asbp_character_base))
      (return true))
    (:CastFailed
      (return false))))

(fn ReceivedNotifyEnd
  (params (MeshComp :type Skeletal%20Mesh%20Component%20Object%20Reference) (Animation :type Anim%20Sequence%20Base%20Object%20Reference))
  (bind _asbp_character_base (Utilities|Casting|CastToBP_Character_Base (Components|GetOwner MeshComp))
    (:then
      (Class|MovementComponent|SetPlaneConstraintNormal (Variables|/Script/Engine.Character|GetCharacterMovement _asbp_character_base) "0, 0, 0")
      (return true))
    (:CastFailed
      (return false))))