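; Actor component that spawns a BP_DamageController for attacks made by its owning BP_Character_Base.
; On authority, CreatDamageController stores the damage data and builds a transform from the mesh socket location and the character's yaw and scale.
; It passes that, with attack time, target and damage value, to the Mult event, which spawns the controller.
; It then resets the character's current attack time.
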(event Custom|CreatDamageController
  (params (DamageData :type Array%20of%20S%20Damage%20Data%20Structures))
  (bind _returnvalue (Components|GetOwner))
  (if (Ability|HasAuthority _returnvalue)
    (Variables|Default|SetDamageDataArray DamageData)
    (bind _asbp_character_base (Utilities|Casting|CastToBP_Character_Base _returnvalue))
    (CallFunction|MultCreatDamageController (Transformation|GetSocketLocation (Variables|/Script/Engine.Character|GetMesh _asbp_character_base) (Variables|Default|GetSocketName)) (Math|Rotator|MakeRotator 0.0 0.0 (.Yaw (Math|Rotator|BreakRotator (.rotation (Transformation|GetActorTransform _asbp_character_base))))) (.scale (Transformation|GetActorTransform _asbp_character_base)) _asbp_character_base _asbp_character_base (Variables|/Game/Blueprints/Character/BP_Character_Base.BP_Character_Base_C|GetCurrAttackTime _asbp_character_base) (Variables|/Game/Blueprints/Character/BP_Character_Base.BP_Character_Base_C|GetCurrTarget _asbp_character_base) (Variables|/Game/Blueprints/Character/BP_Character_Base.BP_Character_Base_C|GetDamageValue _asbp_character_base) (Variables|Default|GetDamageDataArray))
    (Variables|/Game/Blueprints/Character/BP_Character_Base.BP_Character_Base_C|SetCurrAttackTime _asbp_character_base 0.0)))

(event Custom|Mult_CreatDamageController
  (params (Spawn%20Transform%20Location :type Vector) (Spawn%20Transform%20Rotation :type Rotator) (Spawn%20Transform%20Scale :type Vector) (Owner :type Actor%20Object%20Reference) (DamageFromActor :type Actor%20Object%20Reference) (SaveAttackTime :type Float%20%28single-precision%29) (LockTarget :type Character%20Object%20Reference) (SaveDamageValue :type Float%20%28single-precision%29) (DamageDataArray :type Array%20of%20S%20Damage%20Data%20Structures))
  (Game|SpawnActorfromClass "/Game/Blueprints/BP_DamageController.BP_DamageController_C" (Math|Transform|MakeTransform Spawn%20Transform%20Location Spawn%20Transform%20Rotation Spawn%20Transform%20Scale) "Undefined" Owner DamageFromActor DamageDataArray SaveAttackTime LockTarget SaveDamageValue 0))

(event EventBeginPlay)

(event EventTick
  (params (DeltaSeconds :type Float%20%28single-precision%29)))