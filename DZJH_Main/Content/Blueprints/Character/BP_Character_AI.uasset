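; AI-controlled combat character that extends a parent character class and runs the BT_Character behavior tree when possessed.
; State changes pause the brain outside the normal state (普通), show an execution sphere during break (击破), and stop movement on dodge (闪避).
; Health and mana consumption refresh its W_CharacterBar widget.
; Overrides replace player input with chance-based perfect defense and random diagonal input vectors.
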(event EventBeginPlay
  (|CallParentFunction)
  (bind _asw_character_bar (Utilities|Casting|CastToW_CharacterBar (UserInterface|GetUserWidgetObject (Variables|Default|GetLockWidget))))
  (Variables|/Game/Widget/W_CharacterBar.W_CharacterBar_C|SetCharacter _asw_character_bar self)
  (Pawn|SpawnDefaultController)
  (CallFunction|Initialization)
  (if (> (Utilities|Array|Length (Variables|Default|GetIdleMontages)) 0)
    (Animation|Montage|PlayMontage (Variables|Character|GetMesh) (Utilities|Array|Get(acopy) (Variables|Default|GetIdleMontages)) 1.0 0.0 "Start")))

(event Collision|EventActorBeginOverlap
  (params (OtherActor :type Actor%20Object%20Reference))
  (|CallParentFunction OtherActor))

(event EventTick
  (params (DeltaSeconds :type Float%20%28single-precision%29))
  (|CallParentFunction DeltaSeconds))

(event EventOnCharacterStateBaseChanged
  (params (Leave :type E_CharacterState_Base%20Enum :default "NewEnumerator0") (Enter :type E_CharacterState_Base%20Enum :default "NewEnumerator0"))
  (bind _self self)
  (bind _chujuesphere (Variables|Default|GetChuJueSphere))
  (bind _returnvalue (AI|GetAIController _self))
  (bind _braincomponent (Variables|/Script/AIModule.AIController|GetBrainComponent _returnvalue))
  (|CallParentFunction Leave Enter)
  (Utilities|FlowControl|Sequence
    (:then_0
      (switch Utilities|FlowControl|Switch|SwitchonE_CharacterState_Base Leave
        (:NewEnumerator0
          (AI|Navigation|StopMovement _returnvalue)
          (AI|Logic|StopLogic _braincomponent ""))
        (:NewEnumerator14
          (Development|SetHiddeninGame _chujuesphere true false)
          (Audio|SpawnSoundatLocation "/Game/Res/Sound/Hit/Wav_JiPo_0.Wav_JiPo_0" (Transformation|GetActorLocation) "0, 0, 0" 1.0 1.0 0.0 0 0))))
    (:then_1
      (switch Utilities|FlowControl|Switch|SwitchonE_CharacterState_Base Enter
        (:NewEnumerator0
          (Class|BrainComponent|RestartLogic _braincomponent))
        (:NewEnumerator14
          (Development|SetHiddeninGame _chujuesphere false false))))))

(event EventConsumeHealth
  (params (Consume :type Float%20%28single-precision%29) (IsDamage? :type Boolean))
  (|CallParentFunction Consume IsDamage?)
  (bind _asw_character_bar (Utilities|Casting|CastToW_CharacterBar (UserInterface|GetUserWidgetObject (Variables|Default|GetLockWidget))))
  (Default|RefreshHealth _asw_character_bar))

(event EventConsumeMana
  (params (Consume :type Float%20%28single-precision%29))
  (|CallParentFunction Consume)
  (bind _asw_character_bar (Utilities|Casting|CastToW_CharacterBar (UserInterface|GetUserWidgetObject (Variables|Default|GetLockWidget))))
  (Default|RefreshMana _asw_character_bar))

(event EventOnCharacterStateActionChanged
  (params (Leave :type E_CharacterState_Action%20Enum :default "NewEnumerator0") (Enter :type E_CharacterState_Action%20Enum :default "NewEnumerator0"))
  (|CallParentFunction Leave Enter)
  (Utilities|FlowControl|Sequence
    (:then_0
      (switch Utilities|FlowControl|Switch|SwitchonE_CharacterState_Action Leave))
    (:then_1
      (switch Utilities|FlowControl|Switch|SwitchonE_CharacterState_Action Enter
        (:NewEnumerator7
          (AI|Navigation|StopMovement (AI|GetAIController self)))))))

(event EventPossessed
  (params (NewController :type Controller%20Object%20Reference))
  (bind _returnvalue (AI|GetAIController NewController))
  (Utilities|IsValid _returnvalue
    (:Is%20Valid
      (AI|RunBehaviorTree _returnvalue "/Game/Blueprints/Character/AI/BT_Character.BT_Character"))))

(fn ConstructionScript
  (|CallParentFunction)
  (CallFunction|Initialization))

(fn AutoDefense
  (params (AttackerCombatValue :type Float%20%28single-precision%29))
  (if (and (< (Math|Random|RandomFloatinRange 0.0 1.0) (Variables|Default|GetAutoDefenseChance)) (CallFunction|CanPerfectDefense))
    (return true)
    (else
      (return false))))

(fn RefreshSaveInputVector
  (bind _returnvalue (Math|Random|RandomBool))
  (bind _returnvalue_2 (Math|Float|SelectFloat 1.0 -1.0 _returnvalue))
  (bind _output_get (Variables|Default|SetSaveInputVector (Math|Vector|Normalize (Math|Vector|MakeVector _returnvalue_2 _returnvalue_2 0.0))))
  (return _output_get))