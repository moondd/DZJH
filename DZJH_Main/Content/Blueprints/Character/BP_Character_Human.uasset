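; BP_Character_Human is a human character Blueprint that extends a parent character class with splattered blood on nearby humans.
; When blood decals are created, it runs the parent logic, then sphere-overlaps nearby pawns around itself.
; Each human found gets CreatBodyBloodDecals, which makes one random decal from its six body decal components visible.
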(event Custom|CreatBodyBloodDecals
  (bind _decal1 (Variables|Default|GetDecal1))
  (bind _decal2 (Variables|Default|GetDecal2))
  (bind _decal3 (Variables|Default|GetDecal3))
  (bind _decal4 (Variables|Default|GetDecal4))
  (bind _decal5 (Variables|Default|GetDecal5))
  (bind _decal (Variables|Default|GetDecal))
  (bind _array (Utilities|Array|MakeArray _decal1 _decal2 _decal3 _decal4 _decal5 _decal))
  (Rendering|SetVisibility (Utilities|Array|Get(acopy) _array (Math|Random|RandomIntegerinRange 0 (Utilities|Array|LastIndex _array))) true false))

(event EventBeginPlay
  (|CallParentFunction))

(event Collision|EventActorBeginOverlap
  (params (OtherActor :type Actor%20Object%20Reference))
  (|CallParentFunction OtherActor) ; 此节点被禁用，将不会被调用。\n从引脚连出引线来编译功能。
)

(event EventTick
  (params (DeltaSeconds :type Float%20%28single-precision%29))
  (|CallParentFunction DeltaSeconds) ; 此节点被禁用，将不会被调用。\n从引脚连出引线来编译功能。
)

(event EventCreatBloodDecals
  (|CallParentFunction)
  (bind _outactors (Collision|SphereOverlapActors (Transformation|GetActorLocation) 3e+02 (Utilities|Array|MakeArray "ObjectTypeQuery3") 0))
  (for _array_element _outactors
    (bind _asbp_character_human (Utilities|Casting|CastToBP_Character_Human _array_element))
    (CallFunction|CreatBodyBloodDecals _asbp_character_human)))

(fn ConstructionScript
  (|CallParentFunction))