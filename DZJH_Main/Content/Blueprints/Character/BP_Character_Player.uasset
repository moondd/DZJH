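; Player-controlled action-combat character that turns input into movement, jump, dodge, defense, attack and weapon-skill instructions for its parent class, and creates the HUD bar.
; Attack input resolves to normal, dash, instant or air type, with a timeline separating taps from charged holds.
; Tab locks the nearest visible valid target via sphere and line traces.
; While player-controlled, Tick updates defense, interpolates the spring-arm camera by speed and state, and prints debug state.
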(event Custom|CE_XuLi
  ;[1 1 1] InputAttack
  (CallFunction|InstructAttack (Utilities|Array|Get(acopy) (.SkillMap (Utilities|Struct|BreakS_CharacterData (Variables|Default|GetCharacterData))) 1) :!label _label)
  (Variables|Default|SetAttackID 0)
  (Timeline|InputAttackTime Stop
    (:Finished
      (Variables|Default|SetAttackID 2)
      (if (CallFunction|CanAttack)
        (goto _label)))))

(event EventBeginPlay
  ;[1 1 1] Begin
  (|CallParentFunction)
  (CallFunction|Initialization)
  (bind _returnvalue (UserInterface|CreateWidget "/Game/Widget/W_PlayerCharacterBar.W_PlayerCharacterBar_C" 0 self))
  (UserInterface|Viewport|AddtoPlayerScreen _returnvalue))

(event Collision|EventActorBeginOverlap
  (params (OtherActor :type Actor%20Object%20Reference))
  (|CallParentFunction OtherActor) ; 此节点被禁用，将不会被调用。\n从引脚连出引线来编译功能。
)

(event EventTick
  (params (DeltaSeconds :type Float%20%28single-precision%29))
  ;[1 1 1] Tick
  (|CallParentFunction DeltaSeconds)
  (if (Pawn|IsPlayerControlled)
    (|UpdateDefense
      (:NewParam
        (|UpdateCameraAction)
        (|DebugCharacterState)))))

(event EventCurrTargetIsDeath
  ;[1 1 1] InputTab
  (if (Pawn|IsPlayerControlled)
    (CallFunction|UnLockCurrTarget)
    (else
      (CallFunction|UnLockCurrTarget))))

(event EventDamagefromOther
  (params (DamageData :type S%20Damage%20Data%20Structure) (DamageFrom :type BP%20Character%20Base%20Object%20Reference) (HitType :type E_HitType%20Enum :default "NewEnumerator0") (AttackTime :type Float%20%28single-precision%29) (D_AttackTime :type Float%20%28single-precision%29) (DamageValue :type Float%20%28single-precision%29))
  (|CallParentFunction DamageData DamageFrom HitType AttackTime D_AttackTime DamageValue)
  (if (Pawn|IsPlayerControlled)
    (switch Utilities|FlowControl|Switch|SwitchonE_HitType HitType
      (:NewEnumerator6
        (Camera|PlayWorldCameraShake "/Game/Blueprints/CameraShake/BP_CameraShake_0.BP_CameraShake_0_C" (Transformation|GetWorldLocation (Variables|Default|GetCamera)) 6e+02 0.0 1.0 true)))))

(event EventConsumeHealth
  (params (Consume :type Float%20%28single-precision%29) (IsDamage? :type Boolean))
  (|CallParentFunction Consume IsDamage?))

(event EventInstructLockCurrTarget
  (params (Target :type BP%20Character%20Base%20Object%20Reference))
  ;[1 1 1] InputTab
  (|CallParentFunction Target))

(event EventConsumeEnergy
  (params (Consume :type Float%20%28single-precision%29))
  (|CallParentFunction Consume))

(event EventConsumeMana
  (params (Consume :type Float%20%28single-precision%29))
  (|CallParentFunction Consume))

(event Input|ActionEvents|InputActionAttack
  (params (Key :type Key%20Structure))
  (bind _can_ (CallFunction|CanAttack))
  (bind _characterdata (Variables|Default|GetCharacterData))
  (bind _skillmap (Utilities|Struct|BreakS_CharacterData _characterdata))
  ;[1 1 1] InputAttack
  (:Pressed
    (Utilities|AttackType
      (:普通技
        (Variables|Default|SetAttackID 1 :!label _label)
        (Timeline|InputAttackTime PlayFromStart
          (:Finished
            (Variables|Default|SetAttackID 2)
            (if _can_
              (CallFunction|InstructAttack (Utilities|Array|Get(acopy) _skillmap 1))
              (Variables|Default|SetAttackID 0 :!label _label_2)
              (Timeline|InputAttackTime Stop)))))
      (:冲刺技
        (goto _label))
      (:顺发技
        (CallFunction|InstructAttack (Utilities|Array|Get(acopy) _skillmap 2))
        (goto _label_2))
      (:空中技
        (if _can_ :!label _label_3
          (CallFunction|InstructAttack "Weapon_3_AirAttack")))))
  (:Released
    (Utilities|FlowControl|Sequence
      (:then_0
        (Timeline|InputAttackTime Stop))
      (:then_1
        (if (and (> (Variables|Default|GetAttackID) 0) (< (Variables|Default|GetAttackID) 2))
          (Utilities|AttackType
            (:普通技
              (CallFunction|InstructAttack "None")
              (goto _label_2))
            (:冲刺技
              (CallFunction|InstructAttack (Utilities|Array|Get(acopy) _skillmap))
              (goto _label_2))
            (:顺发技
              (goto _label_2))
            (:空中技
              (goto _label_3)))
          (else
            (goto _label_2)))))))

(event Input|ActionEvents|InputActionJump
  (params (Key :type Key%20Structure))
  ;[1 1 1] InputJump
  (:Pressed
    (CallFunction|InstructJump)))

(event Input|ActionEvents|InputActionDefense
  (params (Key :type Key%20Structure))
  ;[1 1 1] InputDefense
  (:Pressed
    (Variables|Default|SetIsInputDefense? true)
    (CallFunction|InstructPerfectDefense))
  (:Released
    (Variables|Default|SetIsInputDefense? false)))

(event Input|AxisEvents|InputAxisMoveForward
  (params (AxisValue :type Float%20%28single-precision%29))
  ;[1 1 1] InputMove
  (Variables|Default|SetInput_Forward AxisValue)
  (if (CallFunction|CanMove)
    (Pawn|Input|AddMovementInput (Math|Vector|RotateVector (Math|Vector|GetRightVector (Transformation|GetWorldRotation (Variables|Default|GetCamera))) "0,-90.000000, 0") (Variables|Default|GetInput_Forward) false)))

(event Input|AxisEvents|InputAxisMoveRight
  (params (AxisValue :type Float%20%28single-precision%29))
  ;[1 1 1] InputMove
  (Variables|Default|SetInput_Right AxisValue)
  (if (CallFunction|CanMove)
    (Pawn|Input|AddMovementInput (Math|Vector|GetRightVector (Transformation|GetWorldRotation (Variables|Default|GetCamera))) (Variables|Default|GetInput_Right) false)))

(event Input|AxisEvents|InputAxisLookUp
  (params (AxisValue :type Float%20%28single-precision%29))
  ;[1 1 1] InputMouseAxis
  (Pawn|Input|AddControllerPitchInput AxisValue))

(event Input|AxisEvents|InputAxisLookRight
  (params (AxisValue :type Float%20%28single-precision%29))
  ;[1 1 1] InputMouseAxis
  (Pawn|Input|AddControllerYawInput AxisValue))

(event Input|KeyboardEvents|Tab
  (params (Key :type Key%20Structure))
  (bind _returnvalue (Pawn|GetControlRotation :!class /Script/Engine.Pawn))
  (bind _returnvalue_2 (Transformation|GetActorLocation))
  (bind _returnvalue_3 (Math|Vector|GetForwardVector _returnvalue))
  (bind _returnvalue_4 (* _returnvalue_3 2.4e+02))
  (bind (_x _y) (Math|Vector|BreakVector _returnvalue_4))
  (bind _returnvalue_5 (Math|Vector|MakeVector _x _y 8e+01))
  (bind _returnvalue_6 (+ _returnvalue_2 _returnvalue_5))
  ;[1 1 1] InputTab
  (:Pressed
    (bind _outhits (Collision|MultiSphereTraceForObjects _returnvalue_6 (+ _returnvalue_6 (* _returnvalue_3 1.2e+03)) 3.6e+02 (Utilities|Array|MakeArray "ObjectTypeQuery7") false (Utilities|Array|MakeArray (Variables|Default|GetCurrTarget)) "None"))
    (CallFunction|UnLockCurrTarget)
    (CallFunction|SelectCurrTarget _outhits)))

(event Input|KeyboardEvents|LeftShift
  (params (Key :type Key%20Structure))
  ;[1 1 1] InputShift
  (:Pressed
    (Variables|Default|SetIsInputDodge? true)
    (CallFunction|InstructDodge)
    (Variables|Default|SetInputMoveState "NewEnumerator1"))
  (:Released
    (Variables|Default|SetIsInputDodge? false)
    (Variables|Default|SetInputMoveState "NewEnumerator0")))

(event Input|KeyboardEvents|Q
  (params (Key :type Key%20Structure))
  ;[1 1 1] InputQER
  (:Pressed
    (CallFunction|InstructAttack (Utilities|Select :Index (Variables|Default|GetWeaponType) :NewEnumerator0 "Weapon_0_Skill_0" :NewEnumerator2 "Weapon_1_Skill_0" :NewEnumerator1 "None" :NewEnumerator4 "None" :NewEnumerator5 "None" :NewEnumerator6 "None" :NewEnumerator7 "None" :NewEnumerator8 "None" :NewEnumerator9 "None" :NewEnumerator10 "None"))))

(event Input|KeyboardEvents|E
  (params (Key :type Key%20Structure))
  ;[1 1 1] InputQER
  (:Pressed
    (CallFunction|InstructAttack (Utilities|Select :Index (Variables|Default|GetWeaponType) :NewEnumerator0 "Weapon_0_Skill_1" :NewEnumerator2 "Weapon_1_Skill_1" :NewEnumerator1 "None" :NewEnumerator4 "None" :NewEnumerator5 "None" :NewEnumerator6 "None" :NewEnumerator7 "None" :NewEnumerator8 "None" :NewEnumerator9 "None" :NewEnumerator10 "None"))))

(event Input|KeyboardEvents|R
  (params (Key :type Key%20Structure))
  ;[1 1 1] InputQER
  (:Pressed
    (CallFunction|InstructAttack (Utilities|Select :Index (Variables|Default|GetWeaponType) :NewEnumerator0 "Weapon_0_Skill_2" :NewEnumerator2 "Weapon_1_Skill_3" :NewEnumerator1 "None" :NewEnumerator4 "None" :NewEnumerator5 "None" :NewEnumerator6 "None" :NewEnumerator7 "None" :NewEnumerator8 "None" :NewEnumerator9 "None" :NewEnumerator10 "None"))))

(event Input|KeyboardEvents|LeftCtrl
  (params (Key :type Key%20Structure))
  ;[1 1 1] InputCtrl
  (:Pressed
    (Variables|Default|SetInputMoveState "NewEnumerator2"))
  (:Released
    (Variables|Default|SetInputMoveState "NewEnumerator0")))

(event EventOnCharacterStateActionChanged
  (params (Leave :type E_CharacterState_Action%20Enum :default "NewEnumerator0") (Enter :type E_CharacterState_Action%20Enum :default "NewEnumerator0"))
  (|CallParentFunction Leave Enter)
  (Utilities|FlowControl|Sequence
    (:then_0
      (switch Utilities|FlowControl|Switch|SwitchonE_CharacterState_Action Leave))
    (:then_1
      (switch Utilities|FlowControl|Switch|SwitchonE_CharacterState_Action Enter
        (:NewEnumerator0
          (if (Variables|Default|GetIsInputDodge?) :!label _label
            (CallFunction|InstructDodge)))
        (:NewEnumerator4
          (switch int (Variables|Default|GetAttackID)
            (:Default
              (goto _label))
            (:0
              (goto _label))
            (:1
              (goto _label))
            (:2
              (CallFunction|CEXuLi))))
        (:NewEnumerator7
          (Variables|Default|SetIsInputDodge? false))))))

(fn ConstructionScript
  (|CallParentFunction)
  (CallFunction|Initialization)
  (Class|SkinnedMeshComponent|SetMasterPoseComponent (Variables|Default|GetVeil) (Variables|Character|GetMesh) false))

(fn AutoDefense
  (params (AttackerCombatValue :type Float%20%28single-precision%29))
  (if (Pawn|IsPlayerControlled)
    (return false)
    (else
      (return (|CallParentFunction AttackerCombatValue)))))

(fn CanPerfectDefense
  (if (Pawn|IsPlayerControlled)
    (return (and (Variables|Default|GetIsInputDefense?) (|CallParentFunction)))
    (else
      (return (|CallParentFunction)))))

(fn UnLockCurrTarget
  (bind _asbp_character_ai (Utilities|Casting|CastToBP_Character_AI (Variables|Default|GetCurrTarget)))
  (Rendering|SetVisibility (Variables|/Game/Blueprints/Character/BP_Character_AI.BP_Character_AI_C|GetLockWidget _asbp_character_ai) false false)
  (CallFunction|InstructLockCurrTarget)
  (return))

(fn SelectCurrTarget
  (params (NewParam :type Array%20of%20Hit%20Result%20Structures))
  (bind _returnvalue (Transformation|GetActorLocation))
  (bind _newlocalvar_0 (LocalVariables|GetNewLocalVar_0))
  (if (> (Utilities|Array|Length NewParam) 0)
    (for _array_element NewParam
      (bind _asbp_character_base (Utilities|Casting|CastToBP_Character_Base (.HitActor (Collision|BreakHitResult _array_element))))
      (bind _returnvalue_2 (Collision|LineTraceByChannel (+ (Transformation|GetActorLocation) "0, 0,60.000000") (+ (Transformation|GetActorLocation (.HitActor (Collision|BreakHitResult _array_element))) "0, 0,60.000000") "TraceTypeQuery1" false 0 "None"))
      (bind _returnvalue_3 (CallFunction|CanAddDamageTargets _asbp_character_base))
      (if (Math|Boolean|ANDBoolean (not _returnvalue_2) (Utilities|Enum|NotEqual(Enum) (Variables|/Game/Blueprints/Character/BP_Character_Base.BP_Character_Base_C|GetCharacterState_Base _asbp_character_base) "NewEnumerator4") _returnvalue_3)
        (Utilities|Array|Add (LocalVariables|GetNewLocalVar_0) _asbp_character_base)))
    (if (> (Utilities|Array|Length _newlocalvar_0) 0)
      (for _array_element_2 _newlocalvar_0
        (bind _asbp_character_base_2 (Utilities|Casting|CastToBP_Character_Base _array_element_2))
        (Utilities|IsValid (LocalVariables|GetLoc_CharacterBase)
          (:Is%20Valid
            (if (< (Math|Vector|VectorLength (- (Transformation|GetActorLocation _array_element_2) _returnvalue)) (Math|Vector|VectorLength (- (Transformation|GetActorLocation (LocalVariables|GetLoc_CharacterBase)) _returnvalue)))
              (LocalVariables|SetLoc_CharacterBase _asbp_character_base_2)))
          (:Is%20Not%20Valid
            (LocalVariables|SetLoc_CharacterBase _asbp_character_base_2))))
      (CallFunction|InstructLockCurrTarget (LocalVariables|GetLoc_CharacterBase))
      (bind _asbp_character_ai (Utilities|Casting|CastToBP_Character_AI (Variables|Default|GetCurrTarget)))
      (Rendering|SetVisibility (Variables|/Game/Blueprints/Character/BP_Character_AI.BP_Character_AI_C|GetLockWidget _asbp_character_ai) true false))))

(fn IsCurrLockTargetinDistence
  (bind _currtarget (Variables|Default|GetCurrTarget))
  (Utilities|IsValid _currtarget
    (:Is%20Valid
      (if (>= (Math|Vector|VectorLength (- (Transformation|GetActorLocation _currtarget) (Transformation|GetActorLocation))) 5e+03)
        (CallFunction|UnLockCurrTarget)))
    (:Is%20Not%20Valid
      (Development|PrintString "无法计算锁定目标距离" true true "(R=1.000000,G=0.000000,B=0.000000,A=1.000000)"))))

(fn CanAddDamageTargets
  (params (Actor :type Actor%20Object%20Reference))
  (bind _asbp_character_enemy (Utilities|Casting|CastToBP_Character_Enemy Actor)
    (:then
      (return _asbp_character_enemy true))
    (:CastFailed
      (bind (_asbp_character_base _returnvalue) (|CallParentFunction Actor))
      (return _asbp_character_base _returnvalue))))

(fn RefreshSaveInputVector
  (bind _camera (Variables|Default|GetCamera))
  (bind _input_forward (Variables|Default|GetInput_Forward))
  (bind _input_right (Variables|Default|GetInput_Right))
  (bind _currtarget (Variables|Default|GetCurrTarget))
  (bind _returnvalue (Transformation|GetWorldRotation _camera))
  (bind _returnvalue_2 (Math|Rotator|MakeRotator 0.0 0.0 (.yaw _returnvalue)))
  (if (and (== _input_forward 0.0) (== _input_right 0.0))
    (Utilities|IsValid _currtarget
      (:Is%20Valid
        (bind _output_get (Variables|Default|SetSaveInputVector (Math|Vector|Normalize (Math|Rotator|GetRotationXVector (Math|Rotator|FindLookatRotation (Transformation|GetActorLocation) (Transformation|GetActorLocation _currtarget))))))
        (return _output_get))
      (:Is%20Not%20Valid
        (bind _output_get_2 (Variables|Default|SetSaveInputVector (Transformation|GetActorForwardVector)))
        (return _output_get_2)))
    (else
      (bind _output_get_3 (Variables|Default|SetSaveInputVector (+ (* (Math|Vector|GetForwardVector _returnvalue_2) _input_forward) (* (Math|Vector|GetRightVector _returnvalue_2) _input_right))))
      (return _output_get_3))))

(event Custom|SetCameraLagSpeed
  (params (CameraLagSpeed :type Float%20%28single-precision%29) (Speed :type Float%20%28single-precision%29))
  (bind _springarm (Variables|Default|GetSpringArm))
  (Variables|/Script/Engine.SpringArmComponent|SetCameraLagSpeed _springarm (Math|Interpolation|FInterpTo (Variables|/Script/Engine.SpringArmComponent|GetCameraLagSpeed _springarm) CameraLagSpeed (Utilities|Time|GetWorldDeltaSeconds) Speed)))

(event Custom|SetCameraArmLength
  (params (TargetArmLength :type Float%20%28single-precision%29) (Speed :type Float%20%28single-precision%29))
  (bind _springarm (Variables|Default|GetSpringArm))
  (Variables|/Script/Engine.SpringArmComponent|SetTargetArmLength _springarm (Math|Interpolation|FInterpTo (Variables|/Script/Engine.SpringArmComponent|GetTargetArmLength _springarm) TargetArmLength (Utilities|Time|GetWorldDeltaSeconds) Speed)))

(event Custom|SetCameraOffset
  (params (Offset :type Vector) (Speed :type Float%20%28single-precision%29))
  (bind _springarm (Variables|Default|GetSpringArm))
  (Variables|/Script/Engine.SpringArmComponent|SetSocketOffset _springarm (Math|Interpolation|VInterpTo (Variables|/Script/Engine.SpringArmComponent|GetSocketOffset _springarm) Offset (Utilities|Time|GetWorldDeltaSeconds) Speed)))

(event Input|KeyboardEvents|0
  (params (Key :type Key%20Structure))
  (:Pressed
    (Game|OpenLevel(byName) "Level_Inn")))