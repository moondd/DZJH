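; BP_DamageNotify is an animation notify that spawns a damage controller for attacks by BP_Character_Base owners.
; The BP_DamageController appears at the mesh's Bip001 socket, using the owner's yaw and scale.
; It receives the notify's DamageData plus the attacker, current target, attack time and damage value.
; The notify then resets the character's attack time, and returns false for other owner types.
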(fn ReceivedNotify
  (params (MeshComp :type Skeletal%20Mesh%20Component%20Object%20Reference) (Animation :type Anim%20Sequence%20Base%20Object%20Reference))
  (bind _returnvalue (Components|GetOwner MeshComp))
  (bind _returnvalue_2 (Transformation|GetActorTransform _returnvalue))
  (bind _asbp_character_base (Utilities|Casting|CastToBP_Character_Base _returnvalue)
    (:then
      (Game|SpawnActorfromClass "/Game/Blueprints/BP_DamageController.BP_DamageController_C" (Math|Transform|MakeTransform (Transformation|GetSocketLocation (Variables|/Script/Engine.Character|GetMesh _asbp_character_base) "Bip001") (Math|Rotator|MakeRotator 0.0 0.0 (.Yaw (Math|Rotator|BreakRotator (.rotation _returnvalue_2)))) (.scale _returnvalue_2)) "Undefined" _returnvalue _returnvalue (Variables|Default|GetDamageData) (Variables|/Game/Blueprints/Character/BP_Character_Base.BP_Character_Base_C|GetCurrAttackTime _asbp_character_base) (Variables|/Game/Blueprints/Character/BP_Character_Base.BP_Character_Base_C|GetCurrTarget _asbp_character_base) (Variables|/Game/Blueprints/Character/BP_Character_Base.BP_Character_Base_C|GetDamageValue _asbp_character_base) 0)
      (Variables|/Game/Blueprints/Character/BP_Character_Base.BP_Character_Base_C|SetCurrAttackTime _asbp_character_base 0.0)
      (return true))
    (:CastFailed
      (return false))))