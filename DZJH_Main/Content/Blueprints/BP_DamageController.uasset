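; BP_DamageController is a short-lived spawner that emits damage actors from the first entry of its damage data array on BeginPlay, then destroys itself.
; A LoopCount macro drives repeated BP_DamageActor spawns based on that entry's count.
; Each spawn applies the entry's location offset in the controller's rotated frame, adds its RandomRotation, and receives the damage source, data array and saved attack time.
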(event Custom|CreatDamageActor
  (bind _returnvalue (Transformation|GetActorTransform))
  (bind _currdamagedata (Variables|Default|GetCurrDamageData))
  (bind (_lodation _randomrotation) (Utilities|Struct|BreakS_DamageData _currdamagedata))
  (bind (_roll _pitch _yaw) (Math|Rotator|BreakRotator (.rotation _returnvalue)))
  (bind (_roll_2 _pitch_2 _yaw_2) (Math|Rotator|BreakRotator _randomrotation))
  (Game|SpawnActorfromClass "/Game/Blueprints/BP_DamageActor.BP_DamageActor_C" (Math|Transform|MakeTransform (+ (.location _returnvalue) (Math|Vector|RotateVector _lodation (.rotation _returnvalue))) (Math|Rotator|MakeRotator (+ _roll _roll_2) (+ _pitch _pitch_2) (+ _yaw _yaw_2)) (.scale _returnvalue)) "Undefined" self (Variables|Default|GetDamageFromActor) (Variables|Default|GetDamageDataArray) (Variables|Default|GetSaveAttackTime) 0))

(event EventBeginPlay
  (Variables|Default|SetCurrDamageData (Utilities|Array|Get(acopy) (Variables|Default|GetDamageDataArray)))
  (Utilities|LoopCount
    (:Then
      (CallFunction|CreatDamageActor))
    (:Complate
      (Actor|DestroyActor))))

(fn ConstructionScript)