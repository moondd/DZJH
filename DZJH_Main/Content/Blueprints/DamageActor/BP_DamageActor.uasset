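; BP_DamageActor is a networked combat damage actor with four modes: area, homing bullet, ground-snapped and grenade.
; Area modes run delayed sphere overlaps filtered by angle, height and faction, while bullets use timeline homing and damage on overlap.
; The authority derives hit type from target state, defense and attack timing, applies damage, then calls multicast hit effects.
; Execution or impact can spawn a BP_DamageController for chained child damage.
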(event OnComponentBeginOverlap(Sphere)
  (params (OverlappedComponent :type Primitive%20Component%20Object%20Reference) (OtherActor :type Actor%20Object%20Reference) (OtherComp :type Primitive%20Component%20Object%20Reference) (OtherBodyIndex :type Integer) (bFromSweep :type Boolean) (SweepResult :type Hit%20Result%20Structure%20%28by%20ref%29))
  (Networking|SwitchHasAuthority
    (:Authority
      (switch Utilities|FlowControl|Switch|SwitchonE_DamageActorType (Utilities|Struct|BreakS_DamageData (Variables|Default|GetCurrDamageData))
        (:NewEnumerator4
          (bind (_can_ _targetcharacter _fromcharacter) (CallFunction|CanShootDamage OtherActor))
          (if _can_
            (CallFunction|MultonDamageExecuted)
            (Utilities|FlowControl|Delay (Utilities|Struct|BreakS_DamageData (Variables|Default|GetCurrDamageData)))
            (bind _outdamageinfo (CallFunction|DamageExecute _targetcharacter _fromcharacter))
            (if (Utilities|Enum|Equal(Enum) (.hittype _outdamageinfo) "NewEnumerator0")
              (Utilities|FlowControl|Delay 6.0)
              (else
                (Utilities|FlowControl|Delay 0.2)))
            (Actor|DestroyActor)))))))

(event Custom|CreatChildDamageData
  (bind _savecontrollertransform (Variables|Default|GetSaveControllerTransform))
  ;[1 1 1] HasChildDamage
  (if (> (Utilities|Array|Length (Variables|Default|GetDamageDataArray)) 0)
    (Game|SpawnActorfromClass "/Game/Blueprints/BP_DamageController.BP_DamageController_C" (Math|Transform|MakeTransform (Transformation|GetActorLocation) (.rotation _savecontrollertransform) (.scale _savecontrollertransform)) "Undefined" (Components|GetOwner) (Variables|Default|GetDamageDataArray) (Variables|Default|GetSaveAttackTime) (Variables|Default|GetLockTarget) (Variables|Default|GetSaveDamageValue) 0)))

(event Custom|Mult_OnDamageActorHit)

(event Custom|StopBulltTrack
  (bind _currdamagedata (Variables|Default|GetCurrDamageData))
  (bind _projectilemovementcomponent (Variables|Default|GetProjectileMovementComponent))
  (bind _locktarget (Variables|Default|GetLockTarget))
  (bind _track_shootspeed (Utilities|Struct|BreakS_DamageData _currdamagedata))
  (Timeline|BulltTrackTime Stop
    (:Update
      ;[1 1 1] 子弹追踪
      (Utilities|IsValid _locktarget
        (:Is%20Valid
          (Transformation|SetActorRotation (Math|Interpolation|RInterpTo (Transformation|GetActorRotation) (Math|Rotator|FindLookatRotation (Transformation|GetActorLocation) (Transformation|GetSocketLocation (Variables|/Script/Engine.Character|GetMesh _locktarget) "Bip001-Spine2")) (Utilities|Time|GetWorldDeltaSeconds) (Math|Interpolation|FInterpTo (Variables|Default|GetCurrTarckRotSpeed) (.Track_RotSpeed (Utilities|Struct|BreakS_DamageData (Variables|Default|GetCurrDamageData))) (Utilities|Time|GetWorldDeltaSeconds) 64.0))))
        (:Is%20Not%20Valid
          _))
      (Utilities|IsValid _projectilemovementcomponent
        (:Is%20Valid
          (Variables|/Script/Engine.MovementComponent|SetVelocity _projectilemovementcomponent (Math|Vector|RotateVector (Variables|Default|GetSaveBulletVelocity) (Transformation|GetActorRotation))))))
    (:Finished
      ;[1 1 1] 子弹追踪结束
      (if (> _track_shootspeed 0.0)
        (Variables|/Script/Engine.MovementComponent|SetVelocity (Variables|Default|GetProjectileMovementComponent) (* (Transformation|GetActorForwardVector) _track_shootspeed))))))

(event Custom|Mult_OnDamageTarget
  (params (HitTarget :type Actor%20Object%20Reference) (HitType :type E_HitType%20Enum :default "NewEnumerator0"))
  (|击中角色表现 HitTarget HitType))

(event Custom|Mult_OnDamageExecuted
  (Networking|SwitchHasAuthority
    (:Authority
      (CallFunction|CreatChildDamageData))))

(event EventBeginPlay
  (bind _currdamagedata (Variables|Default|GetCurrDamageData))
  (bind _currdamagedata_2 (Variables|Default|GetCurrDamageData))
  (bind _locktarget (Variables|Default|GetLockTarget))
  (bind _track_shootspeed (Utilities|Struct|BreakS_DamageData _currdamagedata))
  (bind (_da_spawndelaytime _da_damagedelaytime _da_spawnlocation _da_randomspawnlocation _da_damagevector _da_minspawnrotation _da_maxspawnrotation _da_minspawnvelocity _da_maxspawnvelocity _track_time _track_rotspeed) (Utilities|Struct|BreakS_DamageData _currdamagedata_2))
  (Utilities|FlowControl|Sequence
    (:then_0
      ;[1 1 1] 基本配置
      (Variables|Default|SetDamageFromActor (Components|GetOwner)))
    (:then_1
      (switch Utilities|FlowControl|Switch|SwitchonE_DamageActorType (Utilities|Struct|BreakS_DamageData (Variables|Default|GetCurrDamageData))
        (:NewEnumerator0
          ;[1 1 1] 范围攻击伤害
          (|范围伤害))
        (:NewEnumerator4
          ;[1 1 1] 子弹逻辑
          (Networking|SwitchHasAuthority
            (:Authority
              (Components|Sphere|SetSphereRadius (Variables|Default|GetSphere) (Utilities|Struct|BreakS_DamageData (Variables|Default|GetCurrDamageData)) true))
            (:Remote
              _))
          (bind _returnvalue (AddComponent|AddProjectileMovementComponent :!label _label))
          (bind _output_get (Variables|Default|SetProjectileMovementComponent _returnvalue))
          (Variables|/Script/Engine.ProjectileMovementComponent|SetMaxSimulationTimeStep _output_get 0.01)
          (if (> _track_time 0.0)
            (Components|Timeline|SetPlayRate (Variables|Default|GetBulltTrackTime) (/ 1.0 _track_time))
            (Timeline|BulltTrackTime PlayFromStart
              (:Update
                ;[1 1 1] 子弹追踪
                (Utilities|IsValid _locktarget
                  (:Is%20Valid
                    (Transformation|SetActorRotation (Math|Interpolation|RInterpTo (Transformation|GetActorRotation) (Math|Rotator|FindLookatRotation (Transformation|GetActorLocation) (Transformation|GetSocketLocation (Variables|/Script/Engine.Character|GetMesh _locktarget) "Bip001-Spine2")) (Utilities|Time|GetWorldDeltaSeconds) (Math|Interpolation|FInterpTo (Variables|Default|GetCurrTarckRotSpeed) _track_rotspeed (Utilities|Time|GetWorldDeltaSeconds) 64.0))))
                  (:Is%20Not%20Valid
                    _))
                (Utilities|IsValid (Variables|Default|GetProjectileMovementComponent) :!label _label_2
                  (:Is%20Valid
                    (Variables|/Script/Engine.MovementComponent|SetVelocity (Variables|Default|GetProjectileMovementComponent) (Math|Vector|RotateVector (Variables|Default|GetSaveBulletVelocity) (Transformation|GetActorRotation))))))
              (:Finished
                ;[1 1 1] 子弹追踪结束
                (if (> _track_shootspeed 0.0)
                  (Variables|/Script/Engine.MovementComponent|SetVelocity (Variables|Default|GetProjectileMovementComponent) (* (Transformation|GetActorForwardVector) _track_shootspeed)))))
            (else
              (goto _label_2))))
        (:NewEnumerator2
          ;[1 1 1] 吸附地面伤害
          (|吸附地面伤害))
        (:NewEnumerator5
          (goto _label))))
    (:then_2
      (Networking|SwitchHasAuthority
        (:Authority
          (Utilities|FlowControl|Delay 9.0)
          (Actor|DestroyActor))))))

(event Collision|EventActorBeginOverlap
  (params (OtherActor :type Actor%20Object%20Reference)))

(event Collision|EventHit
  (params (MyComp :type Primitive%20Component%20Object%20Reference) (Other :type Actor%20Object%20Reference) (OtherComp :type Primitive%20Component%20Object%20Reference) (bSelfMoved :type Boolean) (HitLocation :type Vector :default "0, 0, 0") (HitNormal :type Vector :default "0, 0, 0") (NormalImpulse :type Vector :default "0, 0, 0") (Hit :type Hit%20Result%20Structure%20%28by%20ref%29))
  (bind _returnvalue (Transformation|GetActorTransform))
  (bind _sphere (Variables|Default|GetSphere))
  (Networking|SwitchHasAuthority
    (:Authority
      (CallFunction|CreatChildDamageData))
    (:Remote
      _))
  (switch Utilities|FlowControl|Switch|SwitchonE_DamageActorType (Utilities|Struct|BreakS_DamageData (Variables|Default|GetCurrDamageData))
    (:NewEnumerator4
      (CallFunction|StopBulltTrack)
      (Collision|SetCollisionEnabled (Variables|Default|GetSphere) "NoCollision")
      (Utilities|FlowControl|Delay 3.0)
      (Networking|SwitchHasAuthority :!label _label
        (:Authority
          (Actor|DestroyActor))))
    (:NewEnumerator2
      (goto _label))
    (:NewEnumerator5
      ;[1 1 1] 榴弹伤害
      (Networking|SwitchHasAuthority
        (:Authority
          (Utilities|FlowControl|Delay (Utilities|Struct|BreakS_DamageData (Variables|Default|GetCurrDamageData)))
          (Components|Sphere|SetSphereRadius _sphere (Utilities|Struct|BreakS_DamageData (Variables|Default|GetCurrDamageData)) true)
          (bind (_outactors _returnvalue_2) (Collision|ComponentOverlapActors _sphere (Math|Transform|MakeTransform HitLocation (.rotation _returnvalue) (.scale _returnvalue)) (Utilities|Array|MakeArray "ObjectTypeQuery7") "/Script/Engine.Actor" (Utilities|Array|MakeArray (Variables|Default|GetDamageFromActor))))
          (if _returnvalue_2
            (for _array_element _outactors
              (bind (_returnvalue_3 _outtarget _outfrom) (CallFunction|CanDamage _array_element))
              (if _returnvalue_3
                (CallFunction|DamageExecute _outtarget _outfrom))))
          (Utilities|FlowControl|Delay 0.2)
          (Actor|DestroyActor))))))

(fn ConstructionScript)

(fn FindDamageTarget
  (params (object :type Actor%20Object%20Reference)))

(fn CanDamage
  (params (TargetActor :type Object%20Object%20Reference))
  (bind _returnvalue (Transformation|GetActorLocation))
  (bind _currdamagedata (Variables|Default|GetCurrDamageData))
  (bind (_da_spawndelaytime _da_damagedelaytime _da_spawnlocation _da_randomspawnlocation _da_damagevector _da_minspawnrotation _da_maxspawnrotation _da_minspawnvelocity _da_maxspawnvelocity _track_time _track_rotspeed _track_shootspeed _angle _min_z _max_z) (Utilities|Struct|BreakS_DamageData _currdamagedata))
  (bind _asbp_character_base (Utilities|Casting|CastToBP_Character_Base (Variables|Default|GetDamageFromActor))
    (:then
      (bind _asbp_character_base_2 (Utilities|Casting|CastToBP_Character_Base TargetActor)
        (:then
          (return (Math|Boolean|ANDBoolean (or (Pawn|IsPlayerControlled _asbp_character_base) (Utilities|Array|ContainsItem (Variables|/Game/Blueprints/Character/BP_Character_Base.BP_Character_Base_C|GetEnemyArray _asbp_character_base) _asbp_character_base_2)) (not (Math|Boolean|ORBoolean (Utilities|Enum|Equal(Enum) (Variables|/Game/Blueprints/Character/BP_Character_Base.BP_Character_Base_C|GetCharacterState_Base _asbp_character_base_2) "NewEnumerator4") (Utilities|Enum|Equal(Enum) (Variables|/Game/Blueprints/Character/BP_Character_Base.BP_Character_Base_C|GetCharacterState_Base _asbp_character_base_2) "NewEnumerator15") (Utilities|Enum|Equal(Enum) (Variables|/Game/Blueprints/Character/BP_Character_Base.BP_Character_Base_C|GetCharacterState_Base _asbp_character_base_2) "NewEnumerator24"))) (and (Math|Float|InRange(Float) (Math|Float|Absolute(Float) (.yaw (Math|Rotator|Delta(Rotator) (Math|Rotator|FindLookatRotation _returnvalue (Transformation|GetWorldLocation (Variables|/Script/Engine.Character|GetMesh _asbp_character_base_2))) (Math|Conversions|RotationFromXVector (Transformation|GetActorForwardVector _asbp_character_base))))) 0.0 _angle) (select (<= _max_z 0.0) true (Math|Float|InRange(Float) (- (.Z (Math|Vector|BreakVector (Transformation|GetWorldLocation (Variables|/Script/Engine.Character|GetMesh _asbp_character_base_2)))) (.Z (Math|Vector|BreakVector _returnvalue))) _min_z _max_z)))) _asbp_character_base_2 _asbp_character_base))
        (:CastFailed
          _)))
    (:CastFailed
      _))
  (return false 0 0))

(fn GetHitType
  (params (TargetCharacter :type BP%20Character%20Base%20Object%20Reference) (FromCharacter :type BP%20Character%20Base%20Object%20Reference))
  (bind _saveattacktime (Variables|Default|GetSaveAttackTime))
  (bind _output_get (LocalVariables|SetLoc_TargetCharacter TargetCharacter))
  (bind _output_get_2 (LocalVariables|SetLoc_FromCharacter FromCharacter))
  (LocalVariables|SetLoc_CombatValue (Variables|/Game/Blueprints/Character/BP_Character_Base.BP_Character_Base_C|GetCombatValue _output_get_2))
  (LocalVariables|SetLoc_D_AttackTime (- _saveattacktime (Variables|/Game/Blueprints/Character/BP_Character_Base.BP_Character_Base_C|GetCurrAttackTime _output_get)))
  (LocalVariables|SetLoc_DamageData (Variables|Default|GetCurrDamageData))
  (switch Utilities|FlowControl|Switch|SwitchonE_CharacterState_Base (Variables|/Game/Blueprints/Character/BP_Character_Base.BP_Character_Base_C|GetCharacterState_Base _output_get)
    (:NewEnumerator0
      (if (> (Variables|/Game/Blueprints/Character/BP_Character_Base.BP_Character_Base_C|GetAttackingTrail (LocalVariables|GetLoc_TargetCharacter)) 0) :!label _label
        (if (Utilities|Array|ContainsItem (Utilities|String|ParseIntoArray (Utilities|String|ToString(Name) (Utilities|Array|Get(acopy) (Variables|/Game/Blueprints/Character/BP_Character_Base.BP_Character_Base_C|GetCurrEquipArray (LocalVariables|GetLoc_FromCharacter)))) ",") "Feng")
          (return "NewEnumerator7" 1.0)
          (else
            _))
        (else
          (if (or (> (Variables|/Game/Blueprints/Character/BP_Character_Base.BP_Character_Base_C|GetDefenseTime (LocalVariables|GetLoc_TargetCharacter)) 0.0) (Default|AutoDefense (LocalVariables|GetLoc_TargetCharacter) (LocalVariables|GetLoc_CombatValue))) :!label _label_2
            (if (Math|Boolean|ANDBoolean (Utilities|Enum|Equal(Enum) (.DamageType (Utilities|Struct|BreakS_DamageData (LocalVariables|GetLoc_DamageData))) "NewEnumerator0") (or (<= (Variables|/Game/Blueprints/Character/BP_Character_Base.BP_Character_Base_C|GetCurrEnergy (LocalVariables|GetLoc_FromCharacter)) 0.0) (not (Pawn|IsPlayerControlled (LocalVariables|GetLoc_FromCharacter)))) true (Utilities|Enum|Equal(Enum) (.DamageActorType (Utilities|Struct|BreakS_DamageData (LocalVariables|GetLoc_DamageData))) "NewEnumerator0"))
              (return "NewEnumerator1" (LocalVariables|GetLoc_D_AttackTime))
              (else
                (return "NewEnumerator0" (LocalVariables|GetLoc_D_AttackTime))))
            (elif (<= (Variables|/Game/Blueprints/Character/BP_Character_Base.BP_Character_Base_C|GetDefenseTime (LocalVariables|GetLoc_TargetCharacter)) 0.0)
              _
              (else
                (return "NewEnumerator5" _saveattacktime))))))
      (if (> (LocalVariables|GetLoc_D_AttackTime) 0.0)
        (if (<= (Variables|/Game/Blueprints/Character/BP_Character_Base.BP_Character_Base_C|GetCurrCore (LocalVariables|GetLoc_TargetCharacter)) 0.0) :!label _label_3
          (Utilities|FlowControl|Sequence
            (:then_0
              _)
            (:then_1
              (return "NewEnumerator6" (LocalVariables|GetLoc_D_AttackTime))))
          (else
            (Variables|/Game/Blueprints/Character/BP_Character_Base.BP_Character_Base_C|SetCurrCore (LocalVariables|GetLoc_TargetCharacter) (- (Variables|/Game/Blueprints/Character/BP_Character_Base.BP_Character_Base_C|GetCurrCore (LocalVariables|GetLoc_TargetCharacter)) (Math|Float|SelectFloat 0.0 (LocalVariables|GetLoc_D_AttackTime) (< (LocalVariables|GetLoc_D_AttackTime) 0.0))))
            (return "NewEnumerator10" (LocalVariables|GetLoc_D_AttackTime))))
        (else
          (return "NewEnumerator10" (LocalVariables|GetLoc_D_AttackTime)))))
    (:NewEnumerator1
      (goto _label))
    (:NewEnumerator13
      (return "NewEnumerator8" _saveattacktime))
    (:NewEnumerator14
      (if (Pawn|IsPlayerControlled (LocalVariables|GetLoc_TargetCharacter))
        (return "NewEnumerator8" _saveattacktime)
        (else
          (return "NewEnumerator6" (LocalVariables|GetLoc_D_AttackTime)))))
    (:NewEnumerator4
      (return "NewEnumerator10" 0.0))
    (:NewEnumerator15
      (return "NewEnumerator11" _saveattacktime))
    (:NewEnumerator16
      (goto _label))
    (:NewEnumerator17
      (goto _label_2))
    (:NewEnumerator18
      (goto _label_2))
    (:NewEnumerator19
      (goto _label_2))
    (:NewEnumerator20
      (goto _label_2))
    (:NewEnumerator21
      (goto _label_3))
    (:NewEnumerator22
      (goto _label_2))
    (:NewEnumerator23
      (goto _label_2)))
  (Variables|/Game/Blueprints/Character/BP_Character_Base.BP_Character_Base_C|SetCurrCore (LocalVariables|GetLoc_TargetCharacter) (Utilities|Struct|BreakS_CharacterData (Variables|/Game/Blueprints/Character/BP_Character_Base.BP_Character_Base_C|GetCharacterData (LocalVariables|GetLoc_TargetCharacter)))))

(fn CanShootDamage
  (params (Actor :type Actor%20Object%20Reference))
  (bind _damagedactorarray (Variables|Default|GetDamagedActorArray))
  (bind _damagefromactor (Variables|Default|GetDamageFromActor))
  (if (!= Actor _damagefromactor)
    (if (Utilities|Array|ContainsItem _damagedactorarray Actor)
      _
      (else
        (Utilities|Array|Add _damagedactorarray Actor)
        (bind _asbp_character_base (Utilities|Casting|CastToBP_Character_Base Actor)
          (:then
            (bind _asbp_character_base_2 (Utilities|Casting|CastToBP_Character_Base _damagefromactor)
              (:then
                (return (Utilities|Enum|NotEqual(Enum) (Variables|/Game/Blueprints/Character/BP_Character_Base.BP_Character_Base_C|GetCharacterState_Base _asbp_character_base) "NewEnumerator4") _asbp_character_base _asbp_character_base_2))
              (:CastFailed
                _)))
          (:CastFailed
            _)))))
  (return false 0 0))

(fn FindDamageVector
  (params (S_DamageData :type S%20Damage%20Data%20Structure%20%28by%20ref%29) (InTransform :type Transform%20%28by%20ref%29) (DamageTarget :type Actor%20Object%20Reference))
  (bind (_location _rotation) (Math|Transform|BreakTransform InTransform))
  (return (+ (Math|Vector|RotateVector (Utilities|Struct|BreakS_DamageData S_DamageData) _rotation) (Math|Vector|Normalize (- (Transformation|GetActorLocation DamageTarget) _location)))))

(fn DamageExecute
  (params (DamageTarget :type BP%20Character%20Base%20Object%20Reference) (DamageFrom :type BP%20Character%20Base%20Object%20Reference))
  (bind _currdamagedata (Variables|Default|GetCurrDamageData))
  (LocalVariables|SetLoc_DamageTarget DamageTarget)
  (LocalVariables|SetLoc_DamageFrom DamageFrom)
  (Utilities|FlowControl|Sequence
    (:then_0
      (bind (_hittype _d_attacktime) (CallFunction|GetHitType (LocalVariables|GetLoc_DamageTarget) (LocalVariables|GetLoc_DamageFrom)))
      (bind _returnvalue (CallFunction|FindDamageVector _currdamagedata (Transformation|GetActorTransform) (LocalVariables|GetLoc_DamageTarget)))
      (LocalVariables|SetLoc_DamageInfo (Utilities|Struct|MakeS_DamageInfo _currdamagedata _returnvalue _hittype (Variables|Default|GetSaveAttackTime) _d_attacktime (Variables|Default|GetSaveDamageValue))))
    (:then_1
      (Default|DamagefromOther (LocalVariables|GetLoc_DamageTarget) (LocalVariables|GetLoc_DamageFrom) (LocalVariables|GetLoc_DamageInfo)))
    (:then_2
      (CallFunction|MultonDamageTarget (LocalVariables|GetLoc_DamageTarget) (Utilities|Struct|BreakS_DamageInfo (LocalVariables|GetLoc_DamageInfo))))
    (:then_3
      (switch Utilities|FlowControl|Switch|SwitchonE_DamageActorType (Utilities|Struct|BreakS_DamageData (Variables|Default|GetCurrDamageData))
        (:NewEnumerator0
          (Default|DamageSpont (LocalVariables|GetLoc_DamageFrom) (LocalVariables|GetLoc_DamageTarget) (LocalVariables|GetLoc_DamageInfo)))))
    (:then_4
      (return (LocalVariables|GetLoc_DamageInfo)))))