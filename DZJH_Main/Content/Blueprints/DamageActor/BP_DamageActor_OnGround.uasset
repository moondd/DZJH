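; BP_DamageActor_OnGround is a damage actor Blueprint that supplies the visual burst when its damage begins.
; DamageActorBegin spawns a concrete grenade explosion particle effect at the actor's location and rotation, then destroys the Sphere1 component.
; DamageActorSpawn is empty, the default BeginPlay, overlap and Tick events are disabled or empty, and no damage logic appears in this graph.
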(event EventBeginPlay
  (|CallParentFunction) ; 此节点被禁用，将不会被调用。\n从引脚连出引线来编译功能。
)

(event Collision|EventActorBeginOverlap
  (params (OtherActor :type Actor%20Object%20Reference))
  (|CallParentFunction OtherActor) ; 此节点被禁用，将不会被调用。\n从引脚连出引线来编译功能。
)

(event EventTick
  (params (DeltaSeconds :type Float%20%28single-precision%29)))

(event EventDamageActorSpawn)

(event EventDamageActorBegin
  (bind _returnvalue (Transformation|GetActorTransform))
  (bind (_location _rotation) (Math|Transform|BreakTransform _returnvalue))
  (Effects|SpawnEmitteratLocation "/Game/Res/Effect/Grenade/Particles/VFX_GrenadeEXP_concrete.VFX_GrenadeEXP_concrete" _location _rotation)
  (Components|DestroyComponent (Variables|Default|GetSphere1)))

(fn ConstructionScript
  (|CallParentFunction))