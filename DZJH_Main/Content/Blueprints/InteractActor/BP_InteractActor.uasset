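; BP_InteractActor is an interactable actor that tracks whether it is available, in use or spent through an InteractState enum.
; Begin, stop and finish events set that state to 交互中 (interacting), 普通 (normal) or 废弃 (discarded), only on the authority.
; CanInteractive returns true only in the normal state, so a finished actor stays unavailable.
; Player ray enter and leave events are empty stubs.
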(event Custom|InteractFinish
  (Networking|SwitchHasAuthority
    (:Authority
      (Variables|Default|SetInteractState "NewEnumerator2"))))

(event Custom|PlayerRayLeave)

(event Custom|InteractStop
  (Networking|SwitchHasAuthority
    (:Authority
      (Variables|Default|SetInteractState "NewEnumerator0"))))

(event Custom|PlayerRayEnter)

(event Custom|CharacterInstructBegin
  (params (CharacterBase :type BP%20Character%20Base%20Object%20Reference))
  (Networking|SwitchHasAuthority
    (:Authority
      (Variables|Default|SetInteractState "NewEnumerator1"))))

(event EventBeginPlay)

(event Collision|EventActorBeginOverlap
  (params (OtherActor :type Actor%20Object%20Reference)))

(event EventTick
  (params (DeltaSeconds :type Float%20%28single-precision%29)))

(fn ConstructionScript)

(fn CanInteractive
  (switch Utilities|FlowControl|Switch|SwitchonE_InteractState (Variables|Default|GetInteractState)
    (:NewEnumerator0
      (return true))
    (:NewEnumerator1
      _)
    (:NewEnumerator2
      _))
  (return false))