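; Save point interact actor that opens the W_SavePoint widget when a valid, locally controlled character interacts with it.
; CharacterInstruct creates the widget on that player's screen, then runs a retriggerable-delay loop that repeatedly calls SetCharacterExp with a fixed value while a validity check passes.
; Player ray enter and leave defer to the parent, while InteractFinish is overridden empty, so the parent's finish logic never runs.
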(event EventBeginPlay)

(event Collision|EventActorBeginOverlap
  (params (OtherActor :type Actor%20Object%20Reference)))

(event EventTick
  (params (DeltaSeconds :type Float%20%28single-precision%29)))

(event EventPlayerRayEnter
  (|CallParentFunction))

(event EventPlayerRayLeave
  (|CallParentFunction))

(event EventInteractFinish)

(event EventCharacterInstruct
  (params (CharacterBase :type BP%20Character%20Base%20Object%20Reference))
  (Utilities|IsValid CharacterBase
    (:Is%20Valid
      (if (Pawn|IsLocallyControlled CharacterBase)
        (bind _returnvalue (UserInterface|CreateWidget "/Game/Widget/W_SavePoint.W_SavePoint_C"))
        (UserInterface|Viewport|AddtoPlayerScreen _returnvalue)
        (Utilities|FlowControl|RetriggerableDelay 0.1 :!label _label)
        (Utilities|IsValid 0
          (:Is%20Valid
            (Default|SetCharacterExp CharacterBase 1000)
            (goto _label)))))))

(fn ConstructionScript)