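; Anim notify that can chain a character into a forced attack during an animation.
; On authority, it checks each requirement entry in order against the owning BP_Character_Base.
; The first one that passes triggers InstructAttack with a random skill group from that entry and returns true.
; Otherwise it calls AnimNotifyReady on the stored character and returns false.
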(fn ReceivedNotify
  (params (MeshComp :type Skeletal%20Mesh%20Component%20Object%20Reference) (Animation :type Anim%20Sequence%20Base%20Object%20Reference))
  (bind _asbp_character_base (Utilities|Casting|CastToBP_Character_Base (Components|GetOwner MeshComp))
    (:then
      (LocalVariables|SetFromCharacter _asbp_character_base)
      (if (Ability|HasAuthority _asbp_character_base)
        (for _array_element (Variables|Default|GetRequirementSkillArray)
          (bind _iscan_ (CallFunction|CanRequirement (.RequirementArray (Utilities|Struct|BreakS_RequirementSkill _array_element)) (LocalVariables|GetFromCharacter)))
          (if _iscan_
            (Default|InstructAttack (LocalVariables|GetFromCharacter) (Utilities|Array|Get(acopy) (.SkillArray (Utilities|Struct|BreakS_RequirementSkill _array_element)) (Math|Random|RandomIntegerinRange 0 (Utilities|Array|LastIndex (.SkillArray (Utilities|Struct|BreakS_RequirementSkill _array_element))))) true)
            (return _iscan_)))))
    (:CastFailed
      _))
  (Default|AnimNotifyReady (LocalVariables|GetFromCharacter))
  (return false))