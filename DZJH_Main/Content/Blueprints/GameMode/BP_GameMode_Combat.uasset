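; Combat game mode that runs battle rounds between player and enemy teams in spectate (观战), join (参战) or duel (单挑) modes.
; NewCombat destroys existing characters, calls team creation, then possesses the first player character in join and duel, also setting its target in duel.
; AnyCharacterDeath reopens W_Pause five seconds after either team empties.
; Team-creation loops are empty, with spawn, AI setup and team-fill logic left disconnected.
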(event Custom|CreatEnemyTeam
  ;[1 1 1] 创建敌方队伍
  (Utilities|Array|Clear (Variables|Default|GetEnemyTeam))
  (for _index (range 0 0)
    _))

(event Custom|CreatPlayerTeam
  ;[1 1 1] 创建玩家队伍
  (Utilities|Array|Clear (Variables|Default|GetPlayerTeam))
  (switch Utilities|FlowControl|Switch|SwitchonE_CombatMode (Variables|Default|GetCombatMode)
    (:NewEnumerator0
      _)
    (:NewEnumerator1
      _))
  (for _array_element (.CharacterDataArray (Utilities|Struct|BreakS_WorldData (Utilities|Array|Get(acopy) (Variables|/Game/Blueprints/BP_SaveGame.BP_SaveGame_C|GetWorldData (Variables|/Game/Blueprints/BP_GameInstance.BP_GameInstance_C|GetSaveGame (Variables|Default|GetBP_GameInstance))))))
    _))

(event Custom|NewCombat
  (params (Level :type Integer))
  (bind _returnvalue (Game|GetPlayerController 0))
  (bind _playerteam (Variables|Default|GetPlayerTeam))
  (bind _output (Utilities|Array|Get(acopy) _playerteam))
  ;[1 1 1] 新一轮战斗
  (Variables|Default|SetCombatMode (CallFunction|GetCombatMode))
  (CallFunction|PossessCharacter (Variables|Default|GetDefaultPawn) (Game|GetPlayerController 0))
  (bind _outactors (Actor|GetAllActorsOfClass "/Game/Blueprints/Character/BP_Character_Base.BP_Character_Base_C"))
  (for _array_element _outactors
    (Actor|DestroyActor _array_element)
    (Utilities|Array|Clear (Variables|Default|GetPlayerTeam))
    (Utilities|Array|Clear (Variables|Default|GetEnemyTeam)))
  (CallFunction|CreatPlayerTeam)
  (CallFunction|CreatEnemyTeam)
  (for _array_element_2 (Variables|Default|GetPlayerTeam)
    (Variables|/Game/Blueprints/Character/BP_Character_Base.BP_Character_Base_C|SetEnemyArray _array_element_2 (Variables|Default|GetEnemyTeam)))
  (Variables|/Script/Engine.PlayerController|SetbShowMouseCursor _returnvalue false)
  (Input|SetInputModeGameOnly _returnvalue)
  (switch Utilities|FlowControl|Switch|SwitchonE_CombatMode (Variables|Default|GetCombatMode)
    (:NewEnumerator1
      (CallFunction|PossessCharacter _output (Game|GetPlayerController 0) :!label _label))
    (:NewEnumerator2
      (Utilities|FlowControl|Sequence
        (:then_0
          (goto _label))
        (:then_1
          (Variables|/Game/Blueprints/Character/BP_Character_Base.BP_Character_Base_C|SetCurrTarget _output (Utilities|Array|Get(acopy) (Variables|Default|GetEnemyTeam))))))))

(event Custom|ShowPauseUI
  ;[1 1 1] 创建界面
  (bind _returnvalue (UserInterface|CreateWidget "/Game/Widget/W_Pause.W_Pause_C"))
  (UserInterface|Viewport|AddtoPlayerScreen _returnvalue))

(event EventBeginPlay
  ;[1 1 1] Begin
  (|CallParentFunction)
  (Variables|Default|SetDefaultPawn (Game|Player|GetPlayerPawn 0))
  (bind _outactors (Actor|GetAllActorsOfClass "/Script/Engine.PlayerStart"))
  (Variables|Default|SetPlayerStartArray _outactors)
  (CallFunction|ShowPauseUI))

(event EventTick
  (params (DeltaSeconds :type Float%20%28single-precision%29)))

(event EventAnyCharacterDeath
  (params (CharacterBase :type BP%20Character%20Base%20Object%20Reference))
  (bind _playerteam (Variables|Default|GetPlayerTeam))
  (bind _enemyteam (Variables|Default|GetEnemyTeam))
  ;[1 1 1] 角色死亡处理
  (bind _returnvalue (Utilities|Array|RemoveItem _playerteam CharacterBase))
  (if _returnvalue
    (if (<= (Utilities|Array|Length _playerteam) 0)
      (Utilities|FlowControl|Delay 5.0 :!label _label)
      (CallFunction|ShowPauseUI))
    (else
      (bind _returnvalue_2 (Utilities|Array|RemoveItem _enemyteam CharacterBase))
      (if _returnvalue_2
        (if (<= (Utilities|Array|Length _enemyteam) 0)
          (goto _label))))))

(fn ConstructionScript)

(fn CreatCharacter
  (params (Character :type BP%20Character%20AI%20Class%20Reference) (Spawn%20Transform%20Location :type Vector) (Spawn%20Transform%20Rotation :type Rotator) (GuildID :type Integer) (ChildID :type Integer))
  (bind _returnvalue (Game|SpawnActorfromClass Character (Math|Transform|MakeTransform Spawn%20Transform%20Location Spawn%20Transform%20Rotation "1,1,1") "AlwaysSpawn" 0 GuildID ChildID 0)))