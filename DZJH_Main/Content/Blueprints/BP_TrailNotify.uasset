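; Animation notify state that shows a weapon trail on a BP_Character_Base owner for the duration of the notify window.
; Begin increments the character's AttackingTrail counter and starts trails between the EffectBegin and EffectEnd sockets.
; End decrements the counter and ends the trails.
; The LeftHand flag selects the left or right weapon trail component in both events.
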(fn ReceivedNotifyEnd
  (params (MeshComp :type Skeletal%20Mesh%20Component%20Object%20Reference) (Animation :type Anim%20Sequence%20Base%20Object%20Reference))
  (bind _asbp_character_base (Utilities|Casting|CastToBP_Character_Base (Components|GetOwner MeshComp)))
  (Math|Integer|DecrementInt (Variables|/Game/Blueprints/Character/BP_Character_Base.BP_Character_Base_C|GetAttackingTrail _asbp_character_base)
    (:%20%20
      (Effects|Particles|Trails|EndTrails (select (Variables|Default|GetLeftHand?) (Variables|/Game/Blueprints/Character/BP_Character_Base.BP_Character_Base_C|GetWeaponTrail_L _asbp_character_base) (Variables|/Game/Blueprints/Character/BP_Character_Base.BP_Character_Base_C|GetWeaponTrail_R _asbp_character_base)))
      (return false))))

(fn ReceivedNotifyBegin
  (params (MeshComp :type Skeletal%20Mesh%20Component%20Object%20Reference) (Animation :type Anim%20Sequence%20Base%20Object%20Reference) (TotalDuration :type Float%20%28single-precision%29))
  (bind _asbp_character_base (Utilities|Casting|CastToBP_Character_Base (Components|GetOwner MeshComp)))
  (Math|Integer|IncrementInt (Variables|/Game/Blueprints/Character/BP_Character_Base.BP_Character_Base_C|GetAttackingTrail _asbp_character_base)
    (:%20%20
      (Effects|Particles|Trails|BeginTrails (select (Variables|Default|GetLeftHand?) (Variables|/Game/Blueprints/Character/BP_Character_Base.BP_Character_Base_C|GetWeaponTrail_L _asbp_character_base) (Variables|/Game/Blueprints/Character/BP_Character_Base.BP_Character_Base_C|GetWeaponTrail_R _asbp_character_base)) "EffectBegin" "EffectEnd" "ETrailWidthMode_FromCentre" 1.0)
      (return false))))